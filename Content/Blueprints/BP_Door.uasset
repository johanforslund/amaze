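; BP_Door is a door actor that swings open when a GearVR_Char holding at least one key overlaps it.
; The Overlap component's begin event checks the character's key count, then writes it back unchanged, so no key is consumed.
; It then plays the DoorMovement timeline, which sets actor rotation to StartRot plus the track's vector offset.
; The graph never assigns StartRot and has no closing logic.
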(event OnComponentBeginOverlap(Overlap)
  (params (OverlappedComponent :type Primitive%20Component%20Object%20Reference) (OtherActor :type Actor%20Object%20Reference) (OtherComp :type Primitive%20Component%20Object%20Reference) (OtherBodyIndex :type Integer) (bFromSweep :type Boolean) (SweepResult :type Hit%20Result%20Structure%20%28by%20ref%29))
  (bind _startrot (Variables|Default|GetStartRot))
  (bind (_roll _pitch _yaw) (Math|Rotator|BreakRotator _startrot))
  (bind _asgear_vr_char (Utilities|Casting|CastToGearVR_Char OtherActor))
  (if (> (Variables|/Game/Blueprints/GearVR_Char.GearVR_Char_C|GetNumberOfKeys _asgear_vr_char) 0)
    (Variables|/Game/Blueprints/GearVR_Char.GearVR_Char_C|SetNumberOfKeys _asgear_vr_char (Variables|/Game/Blueprints/GearVR_Char.GearVR_Char_C|GetNumberOfKeys _asgear_vr_char))
    (bind _newtrack_0 (Timeline|DoorMovement Play)
      (:Update
        (Transformation|SetActorRotation (Math|Rotator|MakeRotator (.X (Math|Vector|BreakVector (+ _newtrack_0 (Math|Vector|MakeVector _roll _pitch _yaw)))) (.Y (Math|Vector|BreakVector (+ _newtrack_0 (Math|Vector|MakeVector _roll _pitch _yaw)))) (.Z (Math|Vector|BreakVector (+ _newtrack_0 (Math|Vector|MakeVector _roll _pitch _yaw))))))))))

(fn ConstructionScript)